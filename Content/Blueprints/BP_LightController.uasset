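; Light controller that tracks groups of bounce and trigger lights, awarding score and switching event lights as groups complete.
; BeginPlay gathers each group by class and takes UI from BP_MainPlayer.
; Handlers compare counters to group sizes, then clear that group; Await triggers are checked individually.
; AllLightHandler gives a jackpot when all flags are set, but LunchLightHandler sets its flag false, and ResetLight clears lights and state.
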(event Custom|ResetLight
  (for _array_element (Variables|Objects|GetRedBounces)
    (Rendering|Material|SetMaterial (Variables|/Game/Blueprints/Objects/PointObjects/BP_RedPointBounce.BP_RedPointBounce_C|GetCylinder _array_element) 0 "/Game/Assets/Materials/LightMaterials/LightOff.LightOff"))
  (for _array_element_2 (Variables|Objects|GetYellowBounces)
    (Rendering|Material|SetMaterial (Variables|/Game/Blueprints/Objects/PointObjects/BP_YellowPointBounce.BP_YellowPointBounce_C|GetCylinder _array_element_2) 0 "/Game/Assets/Materials/LightMaterials/LightOff.LightOff"))
  (for _array_element_3 (Variables|Objects|GetLunchPadLight)
    (Rendering|Material|SetMaterial (Variables|/Game/Blueprints/Objects/Triggers/LightTrigger/BP_LunchPadLightTrigger.BP_LunchPadLightTrigger_C|GetCone _array_element_3) 0 "/Game/Assets/Materials/LightMaterials/LightOff.LightOff"))
  (for _array_element_4 (Variables|Objects|GetPlaceLight)
    (Rendering|Material|SetMaterial (Variables|/Game/Blueprints/Objects/Triggers/LightTrigger/BP_PlaceLightTrigger.BP_PlaceLightTrigger_C|GetSphere _array_element_4) 0 "/Game/Assets/Materials/LightMaterials/LightOff.LightOff"))
  (for _array_element_5 (Variables|Objects|GetReloadTriggers)
    (Rendering|Material|SetMaterial (Variables|/Game/Blueprints/Objects/Triggers/GameTriggers/BP_ReloadTrigger.BP_ReloadTrigger_C|GetCone _array_element_5) 0 "/Game/Assets/Materials/LightMaterials/LightOff.LightOff"))
  (CallFunction|ResetEventLight)
  (Variables|Counters|SetRedCounter 0)
  (Variables|Counters|SetYellowCounter 0)
  (Variables|Counters|SetPlaceCounter 0)
  (Variables|Counters|SetLunchLightCounter 0)
  (Variables|AllHandler|SetReloadLightOn false)
  (Variables|AllHandler|SetPlaceLightOn false)
  (Variables|AllHandler|SetRedLightOn false)
  (Variables|AllHandler|SetYellowLightOn false)
  (Variables|AllHandler|SetLunchLightOn false)
  (Variables|AllHandler|SetAwaitLight1On false)
  (Variables|AllHandler|SetAwaitLight2On false))

(event Custom|YellowHandler
  (bind _ui (Variables|Components|GetUI))
  (if (== (Variables|Counters|GetYellowCounter) (Variables|Indexes|GetYellowIndex))
    (bind _output_get (Default|AddScore _ui 5000))
    (Default|UpdateScore _ui _output_get)
    (for _array_element (Variables|Objects|GetYellowBounces)
      (Rendering|Material|SetMaterial (Variables|/Game/Blueprints/Objects/PointObjects/BP_YellowPointBounce.BP_YellowPointBounce_C|GetCylinder _array_element) 0 "/Game/Assets/Materials/LightMaterials/LightOff.LightOff")
      (Rendering|Material|SetMaterial (Variables|Default|GetEventYellow) 0 "/Game/Assets/Materials/LightMaterials/LightOn.LightOn")
      (Variables|AllHandler|SetYellowLightOn true)
      (CallFunction|AllLightHandler))
    (Variables|Counters|SetYellowCounter 0)
    (else
      (Development|PrintString "YellowWorked"))))

(event Custom|RedHandle
  (bind _ui (Variables|Components|GetUI))
  (if (== (Variables|Counters|GetRedCounter) (Variables|Indexes|GetRedIndex))
    (bind _output_get (Default|AddScore _ui 5000))
    (Default|UpdateScore _ui _output_get)
    (for _array_element (Variables|Objects|GetRedBounces)
      (Rendering|Material|SetMaterial (Variables|/Game/Blueprints/Objects/PointObjects/BP_RedPointBounce.BP_RedPointBounce_C|GetCylinder _array_element) 0 "/Game/Assets/Materials/LightMaterials/LightOff.LightOff")
      (Rendering|Material|SetMaterial (Variables|Default|GetEventRed) 0 "/Game/Assets/Materials/LightMaterials/LightOn.LightOn")
      (Variables|AllHandler|SetRedLightOn true)
      (CallFunction|AllLightHandler))
    (Variables|Counters|SetRedCounter 0)
    (else
      (Development|PrintString "RedWorked"))))

(event Custom|AwaitHandler
  (for (_array_element _array_index) (Variables|Objects|GetAwaitTriggers)
    (if (and (Variables|/Game/Blueprints/Objects/Triggers/GameTriggers/BP_AwaitTrigger.BP_AwaitTrigger_C|GetbIsOn _array_element) (== _array_index 0))
      (Rendering|Material|SetMaterial (Variables|Default|GetEventAwait1) 0 "/Game/Assets/Materials/LightMaterials/LightOn.LightOn")
      (Variables|AllHandler|SetAwaitLight1On true)
      (CallFunction|AllLightHandler :!label _label)
      (elif (and (Variables|/Game/Blueprints/Objects/Triggers/GameTriggers/BP_AwaitTrigger.BP_AwaitTrigger_C|GetbIsOn _array_element) (== _array_index 1))
        (Rendering|Material|SetMaterial (Variables|Default|GetEventAwait2) 0 "/Game/Assets/Materials/LightMaterials/LightOn.LightOn")
        (Variables|AllHandler|SetAwaitLight2On true)
        (goto _label)))))

(event Custom|PlaceHandler
  (bind _ui (Variables|Components|GetUI))
  (if (== (Variables|Counters|GetPlaceCounter) (Variables|Indexes|GetPlaceIndex))
    (bind _output_get (Default|AddScore _ui 5000))
    (Default|UpdateScore _ui _output_get)
    (for _array_element (Variables|Objects|GetPlaceLight)
      (Rendering|Material|SetMaterial (Variables|/Game/Blueprints/Objects/Triggers/LightTrigger/BP_PlaceLightTrigger.BP_PlaceLightTrigger_C|GetSphere _array_element) 0 "/Game/Assets/Materials/LightMaterials/LightOff.LightOff")
      (Rendering|Material|SetMaterial (Variables|Default|GetEventPlace) 0 "/Game/Assets/Materials/LightMaterials/LightOn.LightOn")
      (Variables|AllHandler|SetPlaceLightOn true)
      (CallFunction|AllLightHandler))
    (Variables|Counters|SetPlaceCounter 0)
    (else
      (Development|PrintString "PlaceWorked"))))

(event Custom|LunchLightHandler
  (bind _ui (Variables|Components|GetUI))
  (if (== (Variables|Counters|GetLunchLightCounter) (Variables|Indexes|GetLunchLightIndex))
    (bind _output_get (Default|AddScore _ui 5000))
    (Default|UpdateScore _ui _output_get)
    (for _array_element (Variables|Objects|GetLunchPadLight)
      (Rendering|Material|SetMaterial (Variables|/Game/Blueprints/Objects/Triggers/LightTrigger/BP_LunchPadLightTrigger.BP_LunchPadLightTrigger_C|GetCone _array_element) 0 "/Game/Assets/Materials/LightMaterials/LightOff.LightOff")
      (Rendering|Material|SetMaterial (Variables|Default|GetEventLunch) 0 "/Game/Assets/Materials/LightMaterials/LightOn.LightOn")
      (Variables|AllHandler|SetLunchLightOn false)
      (CallFunction|AllLightHandler))
    (Variables|Counters|SetLunchLightCounter 0)
    (else
      (Development|PrintString "LunchLightWorked"))))

(event Custom|ReloadLightHandler
  (bind _ui (Variables|Components|GetUI))
  (if (== (Variables|Counters|GetReloadLightCounter) (Variables|Indexes|GetReloadLightIndex))
    (bind _output_get (Default|AddScore _ui 5000))
    (Default|UpdateScore _ui _output_get)
    (for _array_element (Variables|Objects|GetReloadTriggers)
      (Rendering|Material|SetMaterial (Variables|/Game/Blueprints/Objects/Triggers/GameTriggers/BP_ReloadTrigger.BP_ReloadTrigger_C|GetCone _array_element) 0 "/Game/Assets/Materials/LightMaterials/LightOff.LightOff")
      (Rendering|Material|SetMaterial (Variables|Default|GetEventReload) 0 "/Game/Assets/Materials/LightMaterials/LightOn.LightOn")
      (Variables|AllHandler|SetReloadLightOn true)
      (CallFunction|AllLightHandler))
    (Variables|Counters|SetReloadLightCounter 0)
    (else
      (Development|PrintString "ReloadLight Worked"))))

(event Custom|Reset%20EventLight
  (Rendering|Material|SetMaterial (Variables|Default|GetEventAll) 0 "/Game/Assets/Materials/LightMaterials/LightOff.LightOff"))

(event Custom|AllLightHandler
  (if (Math|Boolean|ANDBoolean (Variables|AllHandler|GetReloadLightOn) (Variables|AllHandler|GetPlaceLightOn) (Variables|AllHandler|GetRedLightOn) (Variables|AllHandler|GetYellowLightOn) (Variables|AllHandler|GetLunchLightOn) (Variables|AllHandler|GetAwaitLight1On) (Variables|AllHandler|GetAwaitLight2On))
    (Rendering|Material|SetMaterial (Variables|Default|GetEventAll) 0 "/Game/Assets/Materials/LightMaterials/LightOff.LightOff")
    (bind _foundwidgets (Widget|GetAllWidgetsOfClass "/Game/HUD/Score.Score_C" true))
    (bind _output_get (Default|AddScore (Utilities|Array|Get(acopy) _foundwidgets) 500000))
    (Default|UpdateScore (Utilities|Array|Get(acopy) _foundwidgets) _output_get)
    (else
      (Development|PrintString "AllHandlerWorked"))))

(event EventBeginPlay
  (CallFunction|InitLight)
  (bind _returnvalue (Actor|GetActorOfClass "/Game/Blueprints/BP_MainPlayer.BP_MainPlayer_C"))
  (Variables|Components|SetUI (Variables|/Game/Blueprints/BP_MainPlayer.BP_MainPlayer_C|GetUI _returnvalue)))

(fn ConstructionScript)

(fn InitLight
  (bind _outactors (Actor|GetAllActorsOfClass "/Game/Blueprints/Objects/PointObjects/BP_RedPointBounce.BP_RedPointBounce_C"))
  (bind _output_get (Variables|Objects|SetRedBounces _outactors))
  (Variables|Indexes|SetRedIndex (Utilities|Array|Length _output_get))
  (bind _outactors_2 (Actor|GetAllActorsOfClass "/Game/Blueprints/Objects/PointObjects/BP_YellowPointBounce.BP_YellowPointBounce_C"))
  (bind _output_get_2 (Variables|Objects|SetYellowBounces _outactors_2))
  (Variables|Indexes|SetYellowIndex (Utilities|Array|Length _output_get_2))
  (bind _outactors_3 (Actor|GetAllActorsOfClass "/Game/Blueprints/Objects/Triggers/LightTrigger/BP_LunchPadLightTrigger.BP_LunchPadLightTrigger_C"))
  (bind _output_get_3 (Variables|Objects|SetLunchPadLight _outactors_3))
  (Variables|Indexes|SetLunchLightIndex (Utilities|Array|Length _output_get_3))
  (bind _outactors_4 (Actor|GetAllActorsOfClass "/Game/Blueprints/Objects/Triggers/LightTrigger/BP_PlaceLightTrigger.BP_PlaceLightTrigger_C"))
  (bind _output_get_4 (Variables|Objects|SetPlaceLight _outactors_4))
  (Variables|Indexes|SetPlaceIndex (Utilities|Array|Length _output_get_4))
  (bind _outactors_5 (Actor|GetAllActorsOfClass "/Game/Blueprints/Objects/Triggers/GameTriggers/BP_ReloadTrigger.BP_ReloadTrigger_C"))
  (bind _output_get_5 (Variables|Objects|SetReloadTriggers _outactors_5))
  (Variables|Indexes|SetReloadLightIndex (Utilities|Array|Length _output_get_5))
  (bind _outactors_6 (Actor|GetAllActorsOfClass "/Game/Blueprints/Objects/Triggers/GameTriggers/BP_AwaitTrigger.BP_AwaitTrigger_C"))
  (Variables|Objects|SetAwaitTriggers _outactors_6))