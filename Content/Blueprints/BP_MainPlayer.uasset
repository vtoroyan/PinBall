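; BP_MainPlayer is the pinball player Blueprint that drives both flippers, the ball launcher and the pause menu.
; BeginPlay caches the Score widget, flippers, launcher, ball and a one-time frame delta.
; Handler events step flipper rotation or launcher pull-back through Delay loops while BP_MainController reports input held, snapping back to rest on release.
; PauseHandler shows the Pause widget, switches to UI-only input and pauses the game.
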(event Custom|RightPinnerDownHandler
  ;[1 1 1] Handle Right pinner working
  (Transformation|SetActorRotation (Variables|Components|GetRight) "54.999664,-89.999908,-90.000031"))

(event Custom|RightPinnerUpHandler
  (bind _right (Variables|Components|GetRight))
  ;[1 1 1] Handle Right pinner working
  (if (< (.roll (Transformation|GetActorRotation _right)) -2e+01) :!label _label
    (Class|Actor|AddActorWorldRotation _right "0.000000, 0,7.000000" true)
    (bind _returnvalue (Actor|GetActorOfClass "/Game/Blueprints/BP_MainController.BP_MainController_C"))
    (if (Variables|/Game/Blueprints/BP_MainController.BP_MainController_C|GetbIsPressedPinner _returnvalue)
      (Utilities|FlowControl|Delay (Variables|Default|GetDeltaSecond))
      (goto _label)
      (else
        (Transformation|SetActorRotation _right "54.999664,-89.999908,-90.000031")))))

(event Custom|LeftPinnerUpHandler
  (bind _left (Variables|Components|GetLeft))
  ;[1 1 1] Handle left pinner working
  (if (> (.roll (Transformation|GetActorRotation _left)) 8e+01) :!label _label
    (Class|Actor|AddActorWorldRotation _left "0.000000, 0,-7.000000" true)
    (bind _returnvalue (Actor|GetActorOfClass "/Game/Blueprints/BP_MainController.BP_MainController_C"))
    (if (Variables|/Game/Blueprints/BP_MainController.BP_MainController_C|GetbIsPressedPinner _returnvalue)
      (Utilities|FlowControl|Delay (Variables|Default|GetDeltaSecond))
      (goto _label)
      (else
        (Transformation|SetActorRotation _left "54.999805,89.999985,89.999916")))))

(event Custom|LeftPinnerDownHandler
  ;[1 1 1] Handle left pinner working
  (Transformation|SetActorRotation (Variables|Components|GetLeft) "54.999805,89.999985,89.999916"))

(event Custom|BallLunchPressedHandler
  (bind _coil_default (Variables|Components|GetCoil_Default))
  ;[1 1 1] Handle BallLunch working
  (if (> (.z (Variables|Components|GetCurrent_Coil)) 3e+02) :!label _label
    (Transformation|AddActorWorldOffset (Variables|Components|GetBallLunch) "0, 0,-1.000000" true)
    (Variables|Components|SetCurrent_Coil (Math|Vector|MakeVector (.x (Variables|Components|GetCurrent_Coil)) (.y (Variables|Components|GetCurrent_Coil)) (- (.z (Variables|Components|GetCurrent_Coil)) 1.0)))
    (bind _returnvalue (Actor|GetActorOfClass "/Game/Blueprints/BP_MainController.BP_MainController_C"))
    (if (Variables|/Game/Blueprints/BP_MainController.BP_MainController_C|GetbIsPressedSpace _returnvalue)
      (Utilities|FlowControl|Delay (Variables|Default|GetDeltaSecond))
      (goto _label)
      (else
        (Transformation|SetActorLocation (Variables|Components|GetBallLunch) _coil_default true false)
        (Variables|Components|SetCurrent_Coil _coil_default)))))

(event Custom|BallLunchUnPressedHandler
  (bind _coil_default (Variables|Components|GetCoil_Default))
  ;[1 1 1] Handle BallLunch working
  (Transformation|SetActorLocation (Variables|Components|GetBallLunch) _coil_default true false)
  (Variables|Components|SetCurrent_Coil _coil_default))

(event Custom|PauseHandler
  (bind _returnvalue (Game|GetPlayerController 0))
  ;[1 1 1] Handle Pause Event
  (bind _foundwidgets (Widget|GetAllWidgetsOfClass "/Game/HUD/Pause.Pause_C" true))
  (Widget|SetVisibility (Utilities|Array|Get(acopy) _foundwidgets) "Visible")
  (Default|HudHandler (Utilities|Array|Get(acopy) _foundwidgets))
  (Variables|/Script/Engine.PlayerController|SetbShowMouseCursor _returnvalue true)
  (Input|SetInputModeUIOnly _returnvalue (Utilities|Array|Get(acopy) _foundwidgets) "DoNotLock")
  (Game|SetGamePaused true))

(event EventBeginPlay
  ;[1 1 1] Initialize Components
  (bind _foundwidgets (Widget|GetAllWidgetsOfClass "/Game/HUD/Score.Score_C" true))
  (Variables|Components|SetUI (Utilities|Array|Get(acopy) _foundwidgets))
  (CallFunction|InitializeComponents)
  (Variables|Default|SetDeltaSecond (Utilities|Time|GetWorldDeltaSeconds)))

(fn ConstructionScript)

(fn InitializeComponents
  (bind _returnvalue (Actor|GetActorOfClass "/Game/Blueprints/Objects/PlayableObjects/BP_PinnerLeft.BP_PinnerLeft_C"))
  (Variables|Components|SetLeft _returnvalue)
  (bind _returnvalue_2 (Actor|GetActorOfClass "/Game/Blueprints/Objects/PlayableObjects/BP_PinnerRight.BP_PinnerRight_C"))
  (Variables|Components|SetRight _returnvalue_2)
  (bind _returnvalue_3 (Actor|GetActorOfClass "/Game/Blueprints/Objects/PlayableObjects/BP_BallLunch.BP_BallLunch_C"))
  (Variables|Components|SetBallLunch _returnvalue_3)
  (bind _output_get (Variables|Components|SetCoil_Default (Transformation|GetActorLocation (Variables|Components|GetBallLunch))))
  (Variables|Components|SetCurrent_Coil _output_get)
  (bind _returnvalue_4 (Actor|GetActorOfClass "/Game/Blueprints/Objects/BP_PlayerBall.BP_PlayerBall_C"))
  (Variables|Components|SetBall _returnvalue_4))