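; BP_PlayerBall is the player ball, which bounces off certain meshes and awards score.
; BeginPlay caches the UI from BP_MainPlayer.
; On sphere hit, components blocking GameTraceChannel1 push the ball along the normalized hit impulse, scaled by PlayerBounce, and add points to the UI.
; Other hits make the sphere a tick prerequisite of the hit actor if it matches certain references (noted as controllable), otherwise of the hit component.
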(event OnComponentHit(Sphere)
  (params (HitComponent :type Primitive%20Component%20Object%20Reference) (OtherActor :type Actor%20Object%20Reference) (OtherComp :type Primitive%20Component%20Object%20Reference) (NormalImpulse :type Vector :default "0, 0, 0") (Hit :type Hit%20Result%20Structure%20%28by%20ref%29))
  (bind _ui (Variables|Default|GetUI))
  (bind _sphere (Variables|Default|GetSphere))
  ;[1 1 1] Handle if is bounsed Mesh
  (if (Utilities|Enum|Equal(Enum) (Collision|GetCollisionResponsetoChannel OtherComp "ECC_GameTraceChannel1") "ECR_Block")
    (Physics|AddImpulse (Variables|Default|GetSphere) (* (Math|Vector|Normalize NormalImpulse) (* (Variables|Default|GetPlayerBounce) 1e+05)) "None" false)
    (bind _output_get (Default|AddScore _ui 100))
    (Default|UpdateScore _ui _output_get)
    (else
      ;[1 1 1] If controllable Add tich on actor, else on other component
      (if (Math|Boolean|ORBoolean (== OtherActor 0) (== OtherActor 0) (== OtherActor 0))
        (Class|Actor|AddTickPrerequisiteComponent OtherActor _sphere)
        (else
          (Class|ActorComponent|AddTickPrerequisiteComponent OtherComp _sphere))))))

(event EventBeginPlay
  ;[1 1 1] Get UI for score
  (bind _returnvalue (Actor|GetActorOfClass "/Game/Blueprints/BP_MainPlayer.BP_MainPlayer_C"))
  (Variables|Default|SetUI (Variables|/Game/Blueprints/BP_MainPlayer.BP_MainPlayer_C|GetUI _returnvalue)))

(fn ConstructionScript)