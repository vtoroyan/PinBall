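; Trigger actor that lights its sphere when something overlaps its box and reports the placement to the light controller.
; The overlap swaps the sphere from LightOff to LightOn, using the current material as the state check so an already lit sphere is ignored.
; It then finds BP_LightController by class, increments PlaceCounter, calls PlaceHandler and prints the count.
; The overlapping actor is not filtered.
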(event OnComponentBeginOverlap(Box)
  (params (OverlappedComponent :type Primitive%20Component%20Object%20Reference) (OtherActor :type Actor%20Object%20Reference) (OtherComp :type Primitive%20Component%20Object%20Reference) (OtherBodyIndex :type Integer) (bFromSweep :type Boolean) (SweepResult :type Hit%20Result%20Structure%20%28by%20ref%29))
  (if (== (Rendering|Material|GetMaterial (Variables|Default|GetSphere) 0) "/Game/Assets/Materials/LightMaterials/LightOff.LightOff")
    (Rendering|Material|SetMaterial (Variables|Default|GetSphere) 0 "/Game/Assets/Materials/LightMaterials/LightOn.LightOn")
    (bind _returnvalue (Actor|GetActorOfClass "/Game/Blueprints/BP_LightController.BP_LightController_C"))
    (Math|Integer|IncrementInt (Variables|/Game/Blueprints/BP_LightController.BP_LightController_C|GetPlaceCounter _returnvalue)
      (:%20%20
        (Default|PlaceHandler _returnvalue)
        (Development|PrintString (Utilities|String|ToString(Integer) (Variables|/Game/Blueprints/BP_LightController.BP_LightController_C|GetPlaceCounter _returnvalue)))))))

(fn ConstructionScript)