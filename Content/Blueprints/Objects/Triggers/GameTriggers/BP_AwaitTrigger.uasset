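; Ball-holding trigger that awards points when hit, holds the ball briefly, then launches it back out.
; On hit it updates the HUD score, destroys the incoming actor, signals BP_LightController and shows a stand-in sphere.
; After a delay it spawns and impulses a new BP_PlayerBall, briefly disabling box collision to avoid recapture.
; If BP_MainController reports a restart after the delay, it skips the respawn and clears IsOn.
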(event OnComponentHit(Box)
  (params (HitComponent :type Primitive%20Component%20Object%20Reference) (OtherActor :type Actor%20Object%20Reference) (OtherComp :type Primitive%20Component%20Object%20Reference) (NormalImpulse :type Vector :default "0, 0, 0") (Hit :type Hit%20Result%20Structure%20%28by%20ref%29))
  (Variables|Default|SetbIsOn true)
  ;[1 1 1] Get Hud, Add Score, Destroy Ball
  (Utilities|IsValid (Variables|Default|GetUI)
    (:Is%20Valid
      _)
    (:Is%20Not%20Valid
      (bind _returnvalue (Actor|GetActorOfClass "/Game/Blueprints/BP_MainPlayer.BP_MainPlayer_C"))
      (Variables|Default|SetUI (Variables|/Game/Blueprints/BP_MainPlayer.BP_MainPlayer_C|GetUI _returnvalue))))
  (bind _output_get (Default|AddScore (Variables|Default|GetUI) 1000))
  (Default|UpdateScore (Variables|Default|GetUI) _output_get)
  (Variables|Default|SetScoreRes _output_get)
  (Actor|DestroyActor OtherActor)
  (bind _returnvalue_2 (Actor|GetActorOfClass "/Game/Blueprints/BP_LightController.BP_LightController_C"))
  (Default|AwaitHandler _returnvalue_2)
  ;[1 1 1] Simulate existing ball in trigger
  (Rendering|SetVisibility (Variables|Default|GetSphere) true false)
  ;[1 1 1] If restarted do nothing, else continue
  (bind _returnvalue_3 (Actor|GetActorOfClass "/Game/Blueprints/BP_MainController.BP_MainController_C"))
  (Utilities|FlowControl|Delay 3.0)
  (if (Variables|/Game/Blueprints/BP_MainController.BP_MainController_C|GetbIsRestart _returnvalue_3)
    (Variables|Default|SetbIsOn false)
    (else
      ;[1 1 1] Off collision
      (Collision|SetCollisionProfileName (Variables|Default|GetBox) "NoCollision" :!class /Script/Engine.PrimitiveComponent)
      ;[1 1 1] Spawn Ball, Remove illusion ball
      (bind _returnvalue_4 (Game|SpawnActorfromClass "/Game/Blueprints/Objects/BP_PlayerBall.BP_PlayerBall_C" (Math|Transform|MakeTransform (Transformation|GetWorldLocation (Variables|Default|GetBox)) "0, 0, 0" "1,1,1") "Undefined" 0 0))
      (Rendering|SetVisibility (Variables|Default|GetSphere) false false)
      ;[1 1 1] Update Score
      (bind _output_get_2 (Default|AddScore (Variables|Default|GetUI)))
      (Default|UpdateScore (Variables|/Game/Blueprints/Objects/BP_PlayerBall.BP_PlayerBall_C|GetUI _returnvalue_4) _output_get_2)
      ;[1 1 1] Add Impulse on Y0.5, Z-0.5 direction
      (Physics|AddImpulse (Variables|/Game/Blueprints/Objects/BP_PlayerBall.BP_PlayerBall_C|GetSphere _returnvalue_4) (* "0,0.500000,-0.500000" 500000) "None" false)
      ;[1 1 1] Return Collision back
      (Utilities|FlowControl|Delay 1.0)
      (Collision|SetCollisionProfileName (Variables|Default|GetBox) "BlockAll" :!class /Script/Engine.PrimitiveComponent))))

(fn ConstructionScript)