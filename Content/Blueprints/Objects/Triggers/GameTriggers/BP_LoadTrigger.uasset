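; BP_LoadTrigger is a trigger that rewards 1000 points when hit, removes the hitting actor and launches a replacement ball.
; On a Box hit it updates the score through the UI taken from BP_MainPlayer, then destroys the other actor without a class check.
; After a three-second delay, unless BP_MainController flags a restart, it spawns BP_PlayerBall at Spawn, refreshes the score and applies a strong upward impulse.
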(event OnComponentHit(Box)
  (params (HitComponent :type Primitive%20Component%20Object%20Reference) (OtherActor :type Actor%20Object%20Reference) (OtherComp :type Primitive%20Component%20Object%20Reference) (NormalImpulse :type Vector :default "0, 0, 0") (Hit :type Hit%20Result%20Structure%20%28by%20ref%29))
  ;[1 1 1] Get Hud, Add 1000 to current score, Destroy Current Actor
  (Utilities|IsValid (Variables|Default|GetUI)
    (:Is%20Valid
      _)
    (:Is%20Not%20Valid
      (bind _returnvalue (Actor|GetActorOfClass "/Game/Blueprints/BP_MainPlayer.BP_MainPlayer_C"))
      (Variables|Default|SetUI (Variables|/Game/Blueprints/BP_MainPlayer.BP_MainPlayer_C|GetUI _returnvalue))))
  (bind _output_get (Default|AddScore (Variables|Default|GetUI) 1000))
  (Default|UpdateScore (Variables|Default|GetUI) _output_get)
  (Variables|Default|SetScoreRes _output_get)
  (Actor|DestroyActor OtherActor)
  ;[1 1 1] If Game Is Restarted Do nothing, Else Continue
  (bind _returnvalue_2 (Actor|GetActorOfClass "/Game/Blueprints/BP_MainController.BP_MainController_C"))
  (Utilities|FlowControl|Delay 3.0)
  (if (not (Variables|/Game/Blueprints/BP_MainController.BP_MainController_C|GetbIsRestart _returnvalue_2))
    ;[1 1 1] Create New Ball on Spawn
    (bind _returnvalue_3 (Game|SpawnActorfromClass "/Game/Blueprints/Objects/BP_PlayerBall.BP_PlayerBall_C" (Math|Transform|MakeTransform (Transformation|GetWorldLocation (Variables|Default|GetSpawn)) "0, 0, 0" "1,1,1") "Undefined" 0 0))
    ;[1 1 1] Adding To Score
    (bind _output_get_2 (Default|AddScore (Variables|Default|GetUI)))
    (Default|UpdateScore (Variables|Default|GetUI) _output_get_2)
    ;[1 1 1] Add Impulse on up(Z) direction
    (Physics|AddImpulse (Variables|/Game/Blueprints/Objects/BP_PlayerBall.BP_PlayerBall_C|GetSphere _returnvalue_3) (* "0, 0,1.000000" 700000) "None" false)))

(fn ConstructionScript)