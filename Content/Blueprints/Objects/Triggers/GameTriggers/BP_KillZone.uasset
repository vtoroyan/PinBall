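; Kill zone that ends a ball's run: any overlapping actor adds 2000 points and is destroyed.
; After two seconds it resets launch-pad block walls, score and lights.
; Unless the main controller flags a restart, it also spawns a new ball at the launcher.
; That path appends scores beating the last saved entry to the HighScores save and refreshes the scoreboard widget.
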(event OnComponentBeginOverlap(Box)
  (params (OverlappedComponent :type Primitive%20Component%20Object%20Reference) (OtherActor :type Actor%20Object%20Reference) (OtherComp :type Primitive%20Component%20Object%20Reference) (OtherBodyIndex :type Integer) (bFromSweep :type Boolean) (SweepResult :type Hit%20Result%20Structure%20%28by%20ref%29))
  ;[1 1 1] Game Over Logic` Get UI, Add 2000 to score, Destory Ball, Spawn New if needed
  (Utilities|IsValid (Variables|Default|GetUI)
    (:Is%20Valid
      _)
    (:Is%20Not%20Valid
      (bind _returnvalue (Actor|GetActorOfClass "/Game/Blueprints/BP_MainPlayer.BP_MainPlayer_C"))
      (Variables|Default|SetUI (Variables|/Game/Blueprints/BP_MainPlayer.BP_MainPlayer_C|GetUI _returnvalue))))
  (bind _output_get (Default|AddScore (Variables|Default|GetUI) 2000))
  (Default|UpdateScore (Variables|Default|GetUI) _output_get)
  (Actor|DestroyActor OtherActor)
  ;[1 1 1] If Restarted Reset lunch pad and score, else continue
  (bind _returnvalue_2 (Actor|GetActorOfClass "/Game/Blueprints/BP_MainController.BP_MainController_C"))
  (Utilities|FlowControl|Delay 2.0)
  (if (Variables|/Game/Blueprints/BP_MainController.BP_MainController_C|GetbIsRestart _returnvalue_2)
    (CallFunction|ResetLunchPad)
    (Default|ResetScore (Variables|Default|GetUI))
    (Default|ResetLight (Variables|Default|GetLightController))
    (else
      (bind _returnvalue_3 (Actor|GetActorOfClass "/Game/Blueprints/Objects/PlayableObjects/BP_BallLunch.BP_BallLunch_C"))
      (Game|SpawnActorfromClass "/Game/Blueprints/Objects/BP_PlayerBall.BP_PlayerBall_C" (Math|Transform|MakeTransform (Transformation|GetWorldLocation (Actor|GetComponentbyClass _returnvalue_3 "/Script/Engine.SphereComponent")) "0, 0, 0" "1,1,1") "Undefined" 0 0)
      (CallFunction|ResetLunchPad)
      ;[1 1 1] Save Game Logic with reseting score
      (Utilities|IsValid (Variables|Default|GetSaveData)
        (:Is%20Valid
          _)
        (:Is%20Not%20Valid
          (bind _returnvalue_4 (SaveGame|CreateSaveGameObject "/Game/Blueprints/S_ScoreBoard.S_ScoreBoard_C"))
          (Variables|Default|SetSaveData _returnvalue_4)))
      (if (< (Utilities|Array|Get(acopy) (Variables|/Game/Blueprints/S_ScoreBoard.S_ScoreBoard_C|GetScoreBoard (Variables|Default|GetSaveData)) (Utilities|Array|LastIndex (Variables|/Game/Blueprints/S_ScoreBoard.S_ScoreBoard_C|GetScoreBoard (Variables|Default|GetSaveData)))) (Variables|/Game/HUD/Score.Score_C|GetScoreValue (Variables|Default|GetUI)))
        (Utilities|Array|Add (Variables|/Game/Blueprints/S_ScoreBoard.S_ScoreBoard_C|GetScoreBoard (Variables|Default|GetSaveData)) (Variables|/Game/HUD/Score.Score_C|GetScoreValue (Variables|Default|GetUI)))
        (SaveGame|SaveGametoSlot (Variables|Default|GetSaveData) "HighScores")
        (bind _foundwidgets (Widget|GetAllWidgetsOfClass "/Game/HUD/ScoreBoard.ScoreBoard_C" true))
        (Default|SetScore (Utilities|Array|Get(acopy) _foundwidgets)))
      (Default|ResetScore (Variables|Default|GetUI))
      (Default|ResetLight (Variables|Default|GetLightController)))))

(event Custom|Reset%20LunchPad
  ;[1 1 1] Lunch Pad Set Default logic (Look in game over)
  (bind _outactors (Actor|GetAllActorsOfClass "/Game/Blueprints/Objects/PointObjects/BP_LunchPad.BP_LunchPad_C"))
  (Rendering|SetVisibility (Variables|/Game/Blueprints/Objects/PointObjects/BP_LunchPad.BP_LunchPad_C|GetBlockWall (Utilities|Array|Get(acopy) _outactors)) false false)
  (Collision|SetCollisionProfileName (Variables|/Game/Blueprints/Objects/PointObjects/BP_LunchPad.BP_LunchPad_C|GetBlockWall (Utilities|Array|Get(acopy) _outactors 1)) "NoCollision" :!class /Script/Engine.PrimitiveComponent))

(event EventBeginPlay
  ;[1 1 1] Load Game Data
  (bind _returnvalue (SaveGame|LoadGamefromSlot "HighScores"))
  (bind _ass_score_board (Utilities|Casting|CastToS_ScoreBoard _returnvalue))
  (Variables|Default|SetSaveData _ass_score_board)
  (bind _returnvalue_2 (Actor|GetActorOfClass "/Game/Blueprints/BP_LightController.BP_LightController_C"))
  (Variables|Default|SetLightController _returnvalue_2))

(fn ConstructionScript)