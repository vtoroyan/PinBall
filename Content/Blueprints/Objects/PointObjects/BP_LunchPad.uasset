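; BP_LunchPad is a launch pad point object that flings whatever hits it upward and awards score.
; A hit on StandartWall caches the UI from BP_MainPlayer, waits briefly, then applies a large vertical impulse to the other component and updates the score.
; After a second short delay it shows BlockWall and switches it to BlockAll collision to block the pad.
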(event OnComponentHit(StandartWall)
  (params (HitComponent :type Primitive%20Component%20Object%20Reference) (OtherActor :type Actor%20Object%20Reference) (OtherComp :type Primitive%20Component%20Object%20Reference) (NormalImpulse :type Vector :default "0, 0, 0") (Hit :type Hit%20Result%20Structure%20%28by%20ref%29))
  ;[1 1 1] Get UI, Add impulse
  (Utilities|IsValid (Variables|Default|GetUI)
    (:Is%20Valid
      _)
    (:Is%20Not%20Valid
      (bind _returnvalue (Actor|GetActorOfClass "/Game/Blueprints/BP_MainPlayer.BP_MainPlayer_C"))
      (Variables|Default|SetUI (Variables|/Game/Blueprints/BP_MainPlayer.BP_MainPlayer_C|GetUI _returnvalue))))
  (Utilities|FlowControl|Delay 3.0)
  (Physics|AddImpulse OtherComp (* "0, 0,1.000000" 700000) "None" false)
  ;[1 1 1] Add Score
  (bind _output_get (Default|AddScore (Variables|Default|GetUI) 5000))
  (Default|UpdateScore (Variables|Default|GetUI) _output_get)
  ;[1 1 1] Block lunchPad
  (Utilities|FlowControl|Delay 1.0)
  (bind _blockwall (CallFunction|InitComponents))
  (Rendering|SetVisibility _blockwall true false)
  (Collision|SetCollisionProfileName _blockwall "BlockAll" :!class /Script/Engine.PrimitiveComponent))

(fn ConstructionScript)

(fn InitComponents
  (return (Variables|Default|GetBlockWall) (Variables|Default|GetStandartWall)))