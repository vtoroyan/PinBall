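; Main controller for what appears to be a pinball game, turning player input into actions on BP_MainPlayer.
; On BeginPlay it caches the player pawn as BP_MainPlayer.
; Press and release inputs for left and right pinners and ball launch set pressed flags and call matching pawn handlers, with both pinners sharing one flag; Pause also forwards.
; InitializeComponents is an unfinished stub of mostly unwired actor lookups.
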(event EventBeginPlay
  ;[1 1 1] Get main Player
  (bind _asbp_main_player (Utilities|Casting|CastToBP_MainPlayer (Game|Player|GetPlayerPawn 0)))
  (Variables|Components|SetMainPlayer _asbp_main_player))

(event Input|ActionEvents|InputActionPinnerLeft
  (params (Key :type Key%20Structure :default "None"))
  (bind _mainplayer (Variables|Components|GetMainPlayer))
  ;[1 1 1] Left Pinner
  (:Pressed
    (Variables|Components|SetbIsPressedPinner true)
    (Default|LeftPinnerUpHandler _mainplayer))
  (:Released
    (Variables|Components|SetbIsPressedPinner false)
    (Default|LeftPinnerDownHandler _mainplayer)))

(event Input|ActionEvents|InputActionPinnerRight
  (params (Key :type Key%20Structure :default "None"))
  (bind _mainplayer (Variables|Components|GetMainPlayer))
  ;[1 1 1] Right Pinner
  (:Pressed
    (Variables|Components|SetbIsPressedPinner true)
    (Default|RightPinnerUpHandler _mainplayer))
  (:Released
    (Variables|Components|SetbIsPressedPinner false)
    (Default|RightPinnerDownHandler _mainplayer)))

(event Input|ActionEvents|InputActionBallLunch
  (params (Key :type Key%20Structure :default "None"))
  (bind _mainplayer (Variables|Components|GetMainPlayer))
  ;[1 1 1] LunchBar
  (:Pressed
    (Variables|Components|SetbIsPressedSpace true)
    (Default|BallLunchPressedHandler _mainplayer))
  (:Released
    (Variables|Components|SetbIsPressedSpace false)
    (Default|BallLunchUnPressedHandler _mainplayer)))

(event Input|ActionEvents|InputActionPause
  (params (Key :type Key%20Structure :default "None"))
  ;[1 1 1] Pause
  (:Pressed
    (Default|PauseHandler (Variables|Components|GetMainPlayer))))

(fn ConstructionScript)

(fn InitializeComponents
  (Actor|GetActorOfClass "/Game/Blueprints/Objects/PlayableObjects/BP_PinnerLeft.BP_PinnerLeft_C"))